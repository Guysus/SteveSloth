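; Player character Blueprint that handles map access and a selection of five traversal and tool abilities.
; The map input flip-flops the WB_Map widget on screen, disabling movement while open and restoring walking on close.
; Switch input cycles CurrentAbility with wraparound and prints its name; Interact calls the matching ability function through an enum switch.
; A forward line trace and interpolation nodes are left unconnected.
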(event Input|EnhancedActionEvents|EnhancedInputActionIA_MapAccess
  (params (ActionValue :type Boolean) (ElapsedSeconds :type Float%20%28double-precision%29) (TriggeredSeconds :type Float%20%28double-precision%29) (InputAction :type Input%20Action%20Object%20Reference :default "/Game/Inputs/IA_MapAccess.IA_MapAccess"))
  (:Started
    (Utilities|FlowControl|FlipFlop
      (:A
        (bind _returnvalue (UserInterface|CreateWidget "/Game/Blueprints/Widgets/WB_Map.WB_Map_C"))
        (UserInterface|Viewport|AddtoViewport _returnvalue 0)
        (Class|PrimitiveComponent|SetVisibleinSceneCaptureOnly (Variables|Default|GetPlayerMarker) false)
        (Pawn|Components|CharacterMovement|DisableMovement (Variables|Character|GetCharacterMovement))
        (Variables|/Script/Engine.PlayerController|SetbShowMouseCursor (Game|GetPlayerController 0) false))
      (:B
        (Widget|RemovefromParent _returnvalue)
        (Pawn|Components|CharacterMovement|SetMovementMode (Variables|Character|GetCharacterMovement) "MOVE_Walking" 0)))))

(event Input|EnhancedActionEvents|EnhancedInputActionIA_Interact
  (params (ActionValue :type Boolean) (ElapsedSeconds :type Float%20%28double-precision%29) (TriggeredSeconds :type Float%20%28double-precision%29) (InputAction :type Input%20Action%20Object%20Reference :default "/Game/Inputs/IA_Interact.IA_Interact"))
  (switch Utilities|FlowControl|Switch|SwitchonEAbility (Utilities|Enum|ByteToEnumEAbility (Math|Conversions|ToByte(Integer) (Variables|Default|GetCurrentAbility)))
    (:GrapplingHook
      (Class|MyPlayer|GrapplingHook))
    (:ClimbingClaw
      (Class|MyPlayer|ClimbingClaw))
    (:Shovel
      (Class|MyPlayer|Shovel))
    (:Propeller
      (Class|MyPlayer|Propeller))
    (:Magnetic
      (Class|MyPlayer|Magnetic))))

(event Input|EnhancedActionEvents|EnhancedInputActionIA_SwitchAbilities
  (params (ActionValue :type Float%20%28double-precision%29) (ElapsedSeconds :type Float%20%28double-precision%29) (TriggeredSeconds :type Float%20%28double-precision%29) (InputAction :type Input%20Action%20Object%20Reference :default "/Game/Inputs/IA_SwitchAbilities.IA_SwitchAbilities"))
  ;[1 1 1] Switch Abilities Up&Down
  (if (> ActionValue 0.0)
    (if (>= (Variables|Default|GetCurrentAbility) 4)
      (Variables|Default|SetCurrentAbility 0)
      (else
        (Variables|Default|SetCurrentAbility (+ (Variables|Default|GetCurrentAbility) 1))))
    (elif (<= (Variables|Default|GetCurrentAbility) 0)
      (Variables|Default|SetCurrentAbility 4)
      (else
        (Variables|Default|SetCurrentAbility (- (Variables|Default|GetCurrentAbility) 1)))))
  (switch Utilities|FlowControl|Switch|SwitchonEAbility (Utilities|Enum|ByteToEnumEAbility (Math|Conversions|ToByte(Integer) (Variables|Default|GetCurrentAbility)))
    (:GrapplingHook
      (Development|PrintString "GrapplingHook"))
    (:ClimbingClaw
      (Development|PrintString "ClimbingClaw"))
    (:Shovel
      (Development|PrintString "Shovel"))
    (:Propeller
      (Development|PrintString "Propeller"))
    (:Magnetic
      (Development|PrintString "Magnetic"))))

(event EventBeginPlay)

(event Collision|EventActorBeginOverlap
  (params (OtherActor :type Actor%20Object%20Reference)))

(event EventTick
  (params (DeltaSeconds :type Float%20%28single-precision%29)))

(fn ConstructionScript)