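; Sloth player character with five cycled abilities (grappling hook, climbing claw, shovel, propeller, magnet) and a toggleable map widget.
; Interact runs the current ability's forward line or sphere trace and, on its matching actor class, sets state, animation or movement mode.
; Tick re-traces to interpolate grapple and magnet moves, stopping once SetActorLocation succeeds, and keeps climbing aligned to wall normals.
; Shovelling disables input briefly before destroying the mound; swimming has no exit here.
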(event Custom|Stop%20Climbing
  (bind _charactermovement (Variables|Character|GetCharacterMovement))
  ;[1 1 1] Climbing Claw
  ;;[1 1 1] Stop Climbing
  (Variables|Default|SetbIsClimbing false)
  (Pawn|Components|CharacterMovement|SetMovementMode _charactermovement "MOVE_Falling" 0)
  (Variables|/Script/Engine.CharacterMovementComponent|SetbOrientRotationToMovement _charactermovement true)
  (Components|Animation|PlayAnimation (Variables|Character|GetMesh) "/Game/Animations/Sloth/Sloth_Idle_Anim.Sloth_Idle_Anim" false))

(event Custom|Stop%20Grappling
  ;[1 1 1] Grappling Hook
  ;;[1 1 1] Stop Grappling
  (Variables|Default|SetbIsGrappling false)
  (Components|Animation|PlayAnimation (Variables|Character|GetMesh) "/Game/Animations/Sloth/Sloth_Idle_Anim.Sloth_Idle_Anim" false))

(event Custom|Stop%20Shovelling
  ;[1 1 1] Shovel
  ;;[1 1 1] Stop Shovelling Event
  (Variables|Default|SetbIsDigging false)
  (Input|EnableInput (Game|GetPlayerCharacter 0) (Game|GetPlayerController 0))
  (Components|Animation|PlayAnimation (Variables|Character|GetMesh) "/Game/Animations/Sloth/Sloth_Idle_Anim.Sloth_Idle_Anim" false))

(event Custom|Stop%20Pulling
  ;[1 1 1] Magnetic
  ;;[1 1 1] Stop Pulling
  (Variables|Default|SetbIsPulling false)
  (Components|Animation|PlayAnimation (Variables|Character|GetMesh) "/Game/Animations/Sloth/Sloth_Idle_Anim.Sloth_Idle_Anim" false))

(event Input|EnhancedActionEvents|EnhancedInputActionIA_MapAccess
  (params (ActionValue :type Boolean) (ElapsedSeconds :type Float%20%28double-precision%29) (TriggeredSeconds :type Float%20%28double-precision%29) (InputAction :type Input%20Action%20Object%20Reference :default "/Game/Inputs/IA_MapAccess.IA_MapAccess"))
  ;[1 1 1] Map Access
  (:Started
    (Utilities|FlowControl|FlipFlop
      (:A
        (bind _returnvalue (UserInterface|CreateWidget "/Game/Blueprints/Widgets/WB_Map.WB_Map_C"))
        (UserInterface|Viewport|AddtoViewport _returnvalue 0)
        (Class|PrimitiveComponent|SetVisibleinSceneCaptureOnly (Variables|Default|GetPlayerMarker) false)
        (Pawn|Components|CharacterMovement|DisableMovement (Variables|Character|GetCharacterMovement))
        (Variables|/Script/Engine.PlayerController|SetbShowMouseCursor (Game|GetPlayerController 0) false))
      (:B
        (Widget|RemovefromParent _returnvalue)
        (Pawn|Components|CharacterMovement|SetMovementMode (Variables|Character|GetCharacterMovement) "MOVE_Walking" 0)))))

(event Input|EnhancedActionEvents|EnhancedInputActionIA_Interact
  (params (ActionValue :type Boolean) (ElapsedSeconds :type Float%20%28double-precision%29) (TriggeredSeconds :type Float%20%28double-precision%29) (InputAction :type Input%20Action%20Object%20Reference :default "/Game/Inputs/IA_Interact.IA_Interact"))
  (bind _returnvalue (Transformation|GetActorRotation))
  ;[1 1 1] Interact Ability Functions
  (switch Utilities|FlowControl|Switch|SwitchonEAbility (Utilities|Enum|ByteToEnumEAbility (Math|Conversions|ToByte(Integer) (Variables|Default|GetCurrentAbility)))
    (:GrapplingHook
      (bind (_outhit _was_hit_) (CallFunction|GrappleHookBlueprintFunction))
      ;[1 1 1] Grappling Hook
      ;;[1 1 1] Grappling Hook Function
      (bind _asbp_metal_ring (Utilities|Casting|CastToBP_MetalRing (.HitActor (Collision|BreakHitResult _outhit))))
      (if (and _was_hit_ (== _asbp_metal_ring (.HitActor (Collision|BreakHitResult _outhit))))
        (Variables|Default|SetbIsGrappling true)
        (Components|Animation|PlayAnimation (Variables|Character|GetMesh) "/Game/Animations/Sloth/Sloth_Grappling_Animation.Sloth_Grappling_Animation" (Variables|Default|GetbIsGrappling))))
    (:ClimbingClaw
      (bind (_outhit_2 _hashit_) (CallFunction|ClimbingClawBlueprintFunction))
      ;[1 1 1] Climbing Claw
      ;;[1 1 1] Climbing Function
      (bind _asbp_climbing_rock (Utilities|Casting|CastToBP_ClimbingRock (.HitActor (Collision|BreakHitResult _outhit_2))))
      (if (and _hashit_ (== _asbp_climbing_rock (.HitActor (Collision|BreakHitResult _outhit_2))))
        (Variables|Default|SetbIsClimbing true)
        (Pawn|Components|CharacterMovement|SetMovementMode (Variables|Character|GetCharacterMovement) "MOVE_Flying" 0)
        (Variables|/Script/Engine.CharacterMovementComponent|SetbOrientRotationToMovement (Variables|Character|GetCharacterMovement) false)
        (Transformation|SetActorRotation (Math|Rotator|MakeRotator (.roll _returnvalue) (.pitch _returnvalue) (+ (.yaw (Math|Rotator|MakeRotfromX (.Normal (Collision|BreakHitResult _outhit_2)))) 1.8e+02)))
        (Components|Animation|PlayAnimation (Variables|Character|GetMesh) "/Game/Animations/Sloth/Sloth_Climbing_Wall_Anim.Sloth_Climbing_Wall_Anim" (Variables|Default|GetbIsClimbing))))
    (:Shovel
      (bind (_out_hits _was_hit__2) (CallFunction|ShovelBlueprintFunction))
      ;[1 1 1] Shovel
      ;;[1 1 1] Shovelling Function
      (bind _asbp_dirt_mound (Utilities|Casting|CastToBp_DirtMound (.HitActor (Collision|BreakHitResult _out_hits))))
      (if (and _was_hit__2 (== _asbp_dirt_mound (.HitActor (Collision|BreakHitResult _out_hits))))
        (Variables|Default|SetbIsDigging true)
        (Components|Animation|PlayAnimation (Variables|Character|GetMesh) "/Game/Animations/Sloth/Sloth_Digging_Animation.Sloth_Digging_Animation" (Variables|Default|GetbIsDigging))
        (Input|DisableInput (Game|GetPlayerCharacter 0) (Game|GetPlayerController 0))
        (Utilities|FlowControl|Delay 5.0)
        (Actor|DestroyActor _asbp_dirt_mound)
        (CallFunction|StopShovelling)))
    (:Propeller
      (bind (_out_hit _was_hit__3) (CallFunction|PropellerBlueprintFunction))
      ;[1 1 1] Propeller Function
      (bind _asbp_water_propeller (Utilities|Casting|CastToBP_WaterPropeller (.HitActor (Collision|BreakHitResult _out_hit))))
      (if (and _was_hit__3 (== _asbp_water_propeller (.HitActor (Collision|BreakHitResult _out_hit))))
        (Variables|Default|SetbIsPropelling true)
        (Pawn|Components|CharacterMovement|SetMovementMode (Variables|Character|GetCharacterMovement) "MOVE_Swimming" 0)
        (Components|Animation|PlayAnimation (Variables|Character|GetMesh) "/Game/Animations/Sloth/Sloth_Swimming_Anim.Sloth_Swimming_Anim" true)))
    (:Magnetic
      (bind (_out_hit_2 _was_hit__4) (CallFunction|MagneticBlueprintFunction))
      ;[1 1 1] Magnetic
      ;;[1 1 1] Magnetic Function
      (bind _asbp_metal_box (Utilities|Casting|CastToBP_MetalBox (.HitActor (Collision|BreakHitResult _out_hit_2))))
      (if (and _was_hit__4 (== _asbp_metal_box (.HitActor (Collision|BreakHitResult _out_hit_2))))
        (Variables|Default|SetbIsPulling true)
        (Components|Animation|PlayAnimation (Variables|Character|GetMesh) "/Game/Animations/Sloth/Sloth_GrapplePull_Anim.Sloth_GrapplePull_Anim" (Variables|Default|GetbIsPulling))))))

(event Input|EnhancedActionEvents|EnhancedInputActionIA_SwitchAbilities
  (params (ActionValue :type Float%20%28double-precision%29) (ElapsedSeconds :type Float%20%28double-precision%29) (TriggeredSeconds :type Float%20%28double-precision%29) (InputAction :type Input%20Action%20Object%20Reference :default "/Game/Inputs/IA_SwitchAbilities.IA_SwitchAbilities"))
  ;[1 1 1] Switch Abilities Up&Down
  (if (> ActionValue 0.0)
    (if (>= (Variables|Default|GetCurrentAbility) 4)
      (Variables|Default|SetCurrentAbility 0)
      (else
        (Variables|Default|SetCurrentAbility (+ (Variables|Default|GetCurrentAbility) 1))))
    (elif (<= (Variables|Default|GetCurrentAbility) 0)
      (Variables|Default|SetCurrentAbility 4)
      (else
        (Variables|Default|SetCurrentAbility (- (Variables|Default|GetCurrentAbility) 1)))))
  (switch Utilities|FlowControl|Switch|SwitchonEAbility (Utilities|Enum|ByteToEnumEAbility (Math|Conversions|ToByte(Integer) (Variables|Default|GetCurrentAbility)))
    (:GrapplingHook
      (Development|PrintString "GrapplingHook"))
    (:ClimbingClaw
      (Development|PrintString "ClimbingClaw"))
    (:Shovel
      (Development|PrintString "Shovel"))
    (:Propeller
      (Development|PrintString "Propeller"))
    (:Magnetic
      (Development|PrintString "Magnetic"))))

(event Input|EnhancedActionEvents|EnhancedInputActionIA_ForwardBack
  (params (ActionValue :type Float%20%28double-precision%29) (ElapsedSeconds :type Float%20%28double-precision%29) (TriggeredSeconds :type Float%20%28double-precision%29) (InputAction :type Input%20Action%20Object%20Reference :default "/Game/Inputs/IA_ForwardBack.IA_ForwardBack"))
  ;[1 1 1] Climbing Claw
  ;;[1 1 1] Climbing Movement
  (if (Variables|Default|GetbIsClimbing)
    (Pawn|Input|AddMovementInput (Math|Vector|GetUpVector (Math|Rotator|MakeRotator 0.0 0.0 (.yaw (Pawn|GetControlRotation :!class /Script/Engine.Pawn)))) ActionValue false)))

(event EventBeginPlay)

(event EventTick
  (params (DeltaSeconds :type Float%20%28single-precision%29))
  (bind _returnvalue (Transformation|GetActorRotation))
  (switch Utilities|FlowControl|Switch|SwitchonEAbility (Utilities|Enum|ByteToEnumEAbility (Math|Conversions|ToByte(Integer) (Variables|Default|GetCurrentAbility)))
    (:GrapplingHook
      ;[1 1 1] Grappling Hook Tick Event
      (if (Variables|Default|GetbIsGrappling)
        (bind (_outhit _was_hit_) (CallFunction|GrappleHookBlueprintFunction))
        (if _was_hit_
          (bind _returnvalue_2 (Transformation|SetActorLocation (Math|Interpolation|VInterpTo (Transformation|GetActorLocation) (.Location (Collision|BreakHitResult _outhit)) 0.1 0.3) false false))
          (if _returnvalue_2
            (CallFunction|StopGrappling)))))
    (:ClimbingClaw
      ;[1 1 1] Climbing Claw Tick Event
      (if (Variables|Default|GetbIsClimbing)
        (bind (_outhit_2 _hashit_) (CallFunction|ClimbingClawBlueprintFunction))
        (if _hashit_
          (Transformation|SetActorRotation (Math|Rotator|MakeRotator (.roll _returnvalue) (.pitch _returnvalue) (+ (.yaw (Math|Rotator|MakeRotfromX (.Normal (Collision|BreakHitResult _outhit_2)))) 1.8e+02)))
          (else
            (CallFunction|StopClimbing)))))
    (:Magnetic
      ;[1 1 1] Magnetic Tick Event
      (if (Variables|Default|GetbIsPulling)
        (bind (_out_hit _was_hit__2) (CallFunction|MagneticBlueprintFunction))
        (if _was_hit__2
          (bind _returnvalue_3 (Transformation|SetActorLocation (.HitActor (Collision|BreakHitResult _out_hit)) (Math|Interpolation|VInterpTo (- (.ImpactPoint (Collision|BreakHitResult _out_hit)) "0.000000,30.000000,10.000000") (Transformation|GetActorLocation) 0.1 0.1) false false))
          (if _returnvalue_3
            (CallFunction|StopPulling)))))))

(fn ConstructionScript)

(fn ClimbingClawBlueprintFunction
  (bind _returnvalue (Transformation|GetActorLocation))
  (bind (_outhit _returnvalue_2) (Collision|LineTraceByChannel _returnvalue (+ _returnvalue (* (Math|Vector|GetForwardVector (Transformation|GetActorRotation)) 1e+02)) "TraceTypeQuery1" false 0 "None"))
  (return _outhit _returnvalue_2))

(fn GrappleHookBlueprintFunction
  (bind _returnvalue (Transformation|GetActorLocation))
  (bind (_outhit _returnvalue_2) (Collision|LineTraceByChannel _returnvalue (+ _returnvalue (* (Math|Vector|GetForwardVector (Transformation|GetActorRotation)) 1e+03)) "TraceTypeQuery1" false 0 "None"))
  (return _outhit _returnvalue_2))

(fn ShovelBlueprintFunction
  (bind _returnvalue (Transformation|GetActorLocation))
  (bind (_outhit _returnvalue_2) (Collision|SphereTraceByChannel _returnvalue (+ _returnvalue (* (Math|Vector|GetForwardVector (Transformation|GetActorRotation)) 50)) 5e+01 "TraceTypeQuery1" false 0 "None"))
  (return _outhit _returnvalue_2))

(fn PropellerBlueprintFunction
  (bind _returnvalue (Transformation|GetActorLocation))
  (bind (_outhit _returnvalue_2) (Collision|SphereTraceByChannel _returnvalue (+ _returnvalue (* (Math|Vector|GetForwardVector (Transformation|GetActorRotation)) 100)) 5e+01 "TraceTypeQuery1" false 0 "None"))
  (return _outhit _returnvalue_2))

(fn MagneticBlueprintFunction
  (bind _returnvalue (Transformation|GetActorLocation))
  (bind (_outhit _returnvalue_2) (Collision|LineTraceByChannel _returnvalue (+ _returnvalue (* (Math|Vector|GetForwardVector (Transformation|GetActorRotation)) 1000)) "TraceTypeQuery1" false 0 "None"))
  (return _outhit _returnvalue_2))