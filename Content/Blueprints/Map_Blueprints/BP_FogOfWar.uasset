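; Fog-of-war actor whose PlaceFog event rebuilds the fog as world-space instances on the FogOfWar component.
; It clears existing instances, then uses nested loops over LevelSize spaced by FogGap.
; As written, the Y loop starts and ends at the same negative bound, giving one row, and grid offsets multiply the actor location rather than add to it.
; Nothing in this Blueprint calls PlaceFog.
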(event Custom|PlaceFog
  (bind _levelsize (Variables|Default|GetLevelSize))
  (bind _fog_gap (Variables|Default|Getfog%20Gap))
  (bind _returnvalue (Utilities|Operators|Divide (.y _levelsize) 2.0 _fog_gap))
  (bind _returnvalue_2 (Utilities|Operators|Divide (.x _levelsize) 2.0 _fog_gap))
  (bind _returnvalue_3 (* _returnvalue -1.0))
  (Components|InstancedStaticMesh|ClearInstances (Variables|Default|GetFogOfWar))
  (for _index (range (Math|Float|Truncate (* _returnvalue_2 -1.0)) (Math|Float|Truncate _returnvalue_2))
    (for _index_2 (range (Math|Float|Truncate _returnvalue_3) (Math|Float|Truncate _returnvalue_3))
      (Components|InstancedStaticMesh|AddInstance (Variables|Default|GetFogOfWar) (Math|Transform|MakeTransform (* (Transformation|GetActorLocation) (Math|Vector|MakeVector (* _index_2 (Variables|Default|Getfog%20Gap)) (* _index (Variables|Default|Getfog%20Gap)) 0.0)) "0, 0, 0" "1.000000,1.000000,1.000000") true))))

(event EventBeginPlay)

(event Collision|EventActorBeginOverlap
  (params (OtherActor :type Actor%20Object%20Reference)))

(event EventTick
  (params (DeltaSeconds :type Float%20%28single-precision%29)))

(fn ConstructionScript)