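; Bp_WorldCam is a scene capture camera actor that frames the world area between two corner target actors, apparently for a map.
; Its construction script runs when both targets are valid, moving the actor to their XY midpoint while keeping its own height.
; It then sets the capture component's ortho width to the larger of the X and Y spans between the targets.
; The event graph holds no runtime logic.
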(event EventBeginPlay)

(event Collision|EventActorBeginOverlap
  (params (OtherActor :type Actor%20Object%20Reference)))

(event EventTick
  (params (DeltaSeconds :type Float%20%28single-precision%29)))

(fn ConstructionScript
  (bind _upperlefttarget (Variables|Default|GetUpperleftTarget))
  (bind _lowerrighttarget (Variables|Default|GetLowerRightTarget))
  (bind _upperlefttarget_2 (Variables|Default|GetUpperleftTarget))
  (bind _lowerrighttarget_2 (Variables|Default|GetLowerRightTarget))
  (bind _returnvalue (Transformation|GetActorLocation _lowerrighttarget_2))
  (bind _returnvalue_2 (Transformation|GetActorLocation _upperlefttarget))
  (bind _returnvalue_3 (Transformation|GetActorLocation _lowerrighttarget))
  (bind _returnvalue_4 (Transformation|GetActorLocation _upperlefttarget_2))
  (bind (_x _y) (Math|Vector|BreakVector _returnvalue))
  (bind (_x_2 _y_2) (Math|Vector|BreakVector _returnvalue_4))
  (bind _returnvalue_5 (- _returnvalue_3 _returnvalue_2))
  (bind _returnvalue_6 (/ _returnvalue_5 2.0))
  (bind _returnvalue_7 (+ _returnvalue_2 _returnvalue_6))
  (bind (_x_3 _y_3) (Math|Vector|BreakVector _returnvalue_7))
  ;[0.7449 0.2499 1] Update Ortho Width
  ;;[0.1973 1 0.9702] if both UpperLeft and Lower right target points are valid then set position of the vector to the center of the world
  (Utilities|IsValid (Variables|Default|GetUpperleftTarget)
    (:Is%20Valid
      (Utilities|IsValid (Variables|Default|GetLowerRightTarget)
        (:Is%20Valid
          (Transformation|SetActorLocation (Math|Vector|MakeVector _x_3 _y_3 (.Z (Math|Vector|BreakVector (Transformation|GetActorLocation)))) false true)
          (Variables|/Script/Engine.SceneCaptureComponent2D|SetOrthoWidth (Variables|Default|GetSceneCaptureComponent2D) (Math|Float|Max(Float) (Math|Float|Absolute(Float) (- _x _x_2)) (Math|Float|Absolute(Float) (- _y _y_2)))))))))