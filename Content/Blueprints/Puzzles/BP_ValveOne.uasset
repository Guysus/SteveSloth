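; Puzzle valve one, which spins its crank when operated and then signals BP_CaveEntrance to change its first light.
; An overlap collider reports to the LevelManager instance whether the player is in the valve's area.
; Tick polls the manager's operated flag, set outside this Blueprint, and rotates the crank by frame time.
; After a short Delay, a DoOnce changes the light, clears the operated flag and marks the valve open.
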(event OnComponentBeginOverlap(ActivationCollider)
  (params (OverlappedComponent :type Primitive%20Component%20Object%20Reference) (OtherActor :type Actor%20Object%20Reference) (OtherComp :type Primitive%20Component%20Object%20Reference) (OtherBodyIndex :type Integer) (bFromSweep :type Boolean) (SweepResult :type Hit%20Result%20Structure%20%28by%20ref%29))
  (if (== OtherActor (Variables|Default|GetThePlayer))
    (Variables|Default|SetisInArea true)
    (Class|MyLevelManager|SetValveAreaOne (Variables|Default|GetLevelManager) true)))

(event OnComponentEndOverlap(ActivationCollider)
  (params (OverlappedComponent :type Primitive%20Component%20Object%20Reference) (OtherActor :type Actor%20Object%20Reference) (OtherComp :type Primitive%20Component%20Object%20Reference) (OtherBodyIndex :type Integer))
  (if (== OtherActor (Variables|Default|GetThePlayer))
    (Variables|Default|SetisInArea false)
    (Variables|Default|SetisActiveated false)
    (Class|MyLevelManager|SetValveAreaOne (Variables|Default|GetLevelManager) false)))

(event EventTick
  (params (DeltaSeconds :type Float%20%28single-precision%29))
  (bind _returnvalue (Class|MyLevelManager|GetValveOneOperated (Variables|Default|GetLevelManager)))
  (if _returnvalue
    (Transformation|AddLocalRotation (Variables|Default|GetCrank) (Math|Rotator|MakeRotator 0.0 0.0 (Math|Float|Lerp 0.0 3.6e+02 DeltaSeconds)) false false)
    (Utilities|FlowControl|Delay 0.75)
    (Utilities|FlowControl|DoOnce false
      (:Completed
        (bind _returnvalue_2 (Actor|GetActorOfClass "/Game/Blueprints/Puzzles/BP_CaveEntrance.BP_CaveEntrance_C"))
        (Default|ChangeLightOne _returnvalue_2)
        (Class|MyLevelManager|SetValveOneOperated (Variables|Default|GetLevelManager) false)
        (Class|MyLevelManager|SetValveOneOpen (Variables|Default|GetLevelManager) true)))))

(event EventBeginPlay
  (bind _asbp_the_player (Utilities|Casting|CastToBP_ThePlayer (Game|GetPlayerCharacter 0)))
  (Variables|Default|SetThePlayer _asbp_the_player)
  (Variables|Default|SetisActiveated false)
  (Variables|Default|SetisInArea false)
  (bind _returnvalue (Class|MyLevelManager|GetInstance))
  (bind _output_get (Variables|Default|SetLevelManager _returnvalue))
  (Class|MyLevelManager|SetValveOneOperated _output_get false))

(fn ConstructionScript)