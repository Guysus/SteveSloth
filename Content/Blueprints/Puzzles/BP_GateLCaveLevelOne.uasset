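; Puzzle gate for cave level one that swings open once all three valves are opened.
; On BeginPlay it caches the player and level manager instance, then resets the manager's three valve states to closed after a brief delay.
; Tick polls those states and, when all are open, eases the gate's yaw toward zero with a delta-time lerp, playing the opening sound once through a DoOnce.
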(event EventBeginPlay
  ;[1 1 1] Initialize Everything
  (CallFunction|InitializeVariables)
  (Utilities|FlowControl|Delay 0.1)
  (bind _returnvalue (Class|MyLevelManager|GetInstance))
  (Variables|Default|SetLevelManager _returnvalue)
  (Class|MyLevelManager|SetValveOneOpen (Variables|Default|GetLevelManager) false)
  (Class|MyLevelManager|SetValveTwoOpen (Variables|Default|GetLevelManager) false)
  (Class|MyLevelManager|SetValveThreeOpen (Variables|Default|GetLevelManager) false))

(event EventTick
  (params (DeltaSeconds :type Float%20%28single-precision%29))
  ;[1 1 1] Slowly Open Gate 90 Degrees to the Right when all valves are opened
  (bind _levelmanager (Variables|Default|GetLevelManager)
    (:then
      (if (Math|Boolean|ANDBoolean (Class|MyLevelManager|GetValeOneOpen _levelmanager) (Class|MyLevelManager|GetValeTwoOpen _levelmanager) (Class|MyLevelManager|GetValeThreeOpen _levelmanager))
        (Transformation|SetActorRotation (Math|Rotator|MakeRotator 0.0 0.0 (Math|Float|Lerp (.yaw (Transformation|GetActorRotation)) 0.0 DeltaSeconds)))
        (Utilities|FlowControl|DoOnce false
          (:Completed
            (Audio|PlaySound2D "/Game/Music_and_SFX/SoundEffects/Objects/Gate/GateOpenSFX.GateOpenSFX" 1.0 1.0 0.0 0 0)))))
    (:else)))

(fn ConstructionScript)

(fn InitializeVariables
  (bind _asbp_the_player (Utilities|Casting|CastToBP_ThePlayer (Game|GetPlayerCharacter 0)))
  (Variables|Default|SetThePlayer _asbp_the_player)
  (Variables|Default|SetcanOpen false))