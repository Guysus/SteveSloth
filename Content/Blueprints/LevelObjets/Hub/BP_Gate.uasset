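; BP_Gate is a hub gate that swings open when the player touches it, then loads level one.
; Overlapping its Box with the cached BP_ThePlayer character sets CanOpen and plays a 2D opening sound.
; While CanOpen is set, Tick eases the actor's yaw toward a fixed angle using a DeltaSeconds lerp.
; A Delay inside Tick clears the flag after two seconds and opens LevelOne.
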(event OnComponentBeginOverlap(Box)
  (params (OverlappedComponent :type Primitive%20Component%20Object%20Reference) (OtherActor :type Actor%20Object%20Reference) (OtherComp :type Primitive%20Component%20Object%20Reference) (OtherBodyIndex :type Integer) (bFromSweep :type Boolean) (SweepResult :type Hit%20Result%20Structure%20%28by%20ref%29))
  ;[1 1 1] Check if Player Collided with Gate to Open it
  (if (== OtherActor (Variables|Default|GetThePlayer))
    (Development|PrintString "player hit me")
    (Variables|Default|SetcanOpen true)
    (Audio|PlaySound2D "/Game/Music_and_SFX/SoundEffects/Objects/Gate/GateOpenSFX.GateOpenSFX" 1.0 1.0 0.0 0 0)))

(event EventBeginPlay
  (CallFunction|InitializeVariables))

(event EventTick
  (params (DeltaSeconds :type Float%20%28single-precision%29))
  ;[1 1 1] Slowly Open Gate 90 Degrees to the Right
  (if (Variables|Default|GetcanOpen)
    (Transformation|SetActorRotation (Math|Rotator|MakeRotator 0.0 0.0 (Math|Float|Lerp (.yaw (Transformation|GetActorRotation)) -1e+02 DeltaSeconds)))
    (Utilities|FlowControl|Delay 2.0)
    (Variables|Default|SetcanOpen false)
    (Game|OpenLevel(byObjectReference) "/Game/Levels/LevelOne.LevelOne")))

(fn ConstructionScript)

(fn InitializeVariables
  (bind _asbp_the_player (Utilities|Casting|CastToBP_ThePlayer (Game|GetPlayerCharacter 0)))
  (Variables|Default|SetThePlayer _asbp_the_player)
  (Variables|Default|SetcanOpen false))